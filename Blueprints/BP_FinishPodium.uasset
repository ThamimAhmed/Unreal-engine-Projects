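; BP_FinishPodium is an interactable finish point that resets the player after a timed shooting run.
; Overlapping its trigger enables input and opens a gate, so the Interact action only works while the character stands there.
; Interacting resets shot stats, plays a sound, teleports the character behind a brief loading screen, moves the TargetWall door back, removes the stopwatch widget and notifies HighscoreText that the run finished.
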(event `EnhancedInput|/Game/ThirdPerson/Input/Actions/IA_Interact`
  (params (ActionValue :type Boolean) (ElapsedSeconds :type "Float (double-precision)") (TriggeredSeconds :type "Float (double-precision)") (InputAction :type "InputAction Object Reference" :default "/Game/ThirdPerson/Input/Actions/IA_Interact.IA_Interact"))
  (bind _char_ref (`self.char Ref`))
  (:`Completed`
    (`/Engine/EditorBlueprintResources/StandardMacros.Gate` true :!label _label
      (:`Exit`
        (set `/Game/ThirdPerson/Blueprints/BP_ThirdPersonCharacter.Accuracy` 100.0 _char_ref)
        (set `/Game/ThirdPerson/Blueprints/BP_ThirdPersonCharacter.TotalShotsFired` 0.0 _char_ref)
        (set `/Game/ThirdPerson/Blueprints/BP_ThirdPersonCharacter.ShotsMissed` 0.0 _char_ref)
        (set `/Game/ThirdPerson/Blueprints/BP_ThirdPersonCharacter.ShotCount` 0.0 _char_ref)
        (`GameplayStatics.PlaySoundAtLocation` "/Game/SoundEffects/gameStartSound.gameStartSound" (0.0 0.0 0.0) (struct) 1.0 1.0 0.0 null null null null)
        (bind _returnvalue (`|CreateWidget` "/Game/Widgets/LoadingScreenWidgetScreen.LoadingScreenWidgetScreen_C"))
        (`UserWidget.AddToViewport` _returnvalue 0)
        (`self.K2_SetActorLocation` (`self.Char Ref`) (980.0 1460.0 92.0) false false)
        (`KismetSystemLibrary.Delay` 0.5)
        (`Widget.RemoveFromParent` _returnvalue)
        (bind _returnvalue_2 (`GameplayStatics.GetActorOfClass` "/Game/ThirdPerson/Blueprints/TargetWall.TargetWall_C"))
        (`/Game/ThirdPerson/Blueprints/TargetWall.MoveDoorBack` _returnvalue_2)
        (bind _returnvalue_3 (`GameplayStatics.GetActorOfClass` "/Game/ThirdPerson/Blueprints/BP_StartTimer.BP_StartTimer_C"))
        (`Widget.RemoveFromParent` (`/Game/ThirdPerson/Blueprints/BP_StartTimer.StopWatchWidget Ref` _returnvalue_3))
        (bind _returnvalue_4 (`GameplayStatics.GetActorOfClass` "/Game/ThirdPerson/Blueprints/HighscoreText.HighscoreText_C"))
        (`/Game/ThirdPerson/Blueprints/HighscoreText.Finished` _returnvalue_4)))))

(event `self.trigger.OnComponentBeginOverlap`
  (params (OverlappedComponent :type "PrimitiveComponent Object Reference") (OtherActor :type "Actor Object Reference") (OtherComp :type "PrimitiveComponent Object Reference") (OtherBodyIndex :type Integer) (bFromSweep :type Boolean) (SweepResult :type "HitResult Structure (by ref)"))
  (bind _asbp_third_person_character (cast `/Game/ThirdPerson/Blueprints/BP_ThirdPersonCharacter` OtherActor))
  (set `self.char Ref` _asbp_third_person_character)
  (`self.EnableInput` (`GameplayStatics.GetPlayerController` 0))
  (goto _label :!via `Open`))

(event `self.trigger.OnComponentEndOverlap`
  (params (OverlappedComponent :type "PrimitiveComponent Object Reference") (OtherActor :type "Actor Object Reference") (OtherComp :type "PrimitiveComponent Object Reference") (OtherBodyIndex :type Integer))
  (bind _asbp_third_person_character (cast `/Game/ThirdPerson/Blueprints/BP_ThirdPersonCharacter` OtherActor))
  (set `self.char Ref` _asbp_third_person_character)
  (`self.DisableInput` (`GameplayStatics.GetPlayerController` 0))
  (goto _label :!via `Close`))

(fn `UserConstructionScript`)