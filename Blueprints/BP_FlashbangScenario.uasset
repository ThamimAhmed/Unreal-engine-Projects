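; BP_FlashbangScenario is a trigger-activated shooting scenario that spawns a single target after a flashbang sequence.
; Overlapping the trigger enables input and opens a gate for Interact, while leaving reverses both.
; Interacting resets the character's shot stats, turns the light green, disables input and plays start and warning sounds.
; If flashbang is enabled, it calls FlashbangMessage, then spawns a randomly placed BP_SingleTarget after a delay and turns the light red.
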(event `EnhancedInput|/Game/ThirdPerson/Input/Actions/IA_Interact`
  (params (ActionValue :type Boolean) (ElapsedSeconds :type "Float (double-precision)") (TriggeredSeconds :type "Float (double-precision)") (InputAction :type "InputAction Object Reference" :default "/Game/ThirdPerson/Input/Actions/IA_Interact.IA_Interact"))
  (bind (_returnvalue_x _returnvalue_y _returnvalue_z) (`KismetMathLibrary.BreakVector` (`self.K2_GetActorLocation`)))
  (bind _returnvalue (`GameplayStatics.GetPlayerController` 0))
  (bind _char_ref (`self.char Ref`))
  (:`Completed`
    (`/Engine/EditorBlueprintResources/StandardMacros.Gate` true :!label _label
      (:`Exit`
        (set `/Game/ThirdPerson/Blueprints/BP_ThirdPersonCharacter.Accuracy` 100.0 _char_ref)
        (set `/Game/ThirdPerson/Blueprints/BP_ThirdPersonCharacter.TotalShotsFired` 0.0 _char_ref)
        (set `/Game/ThirdPerson/Blueprints/BP_ThirdPersonCharacter.ShotsMissed` 0.0 _char_ref)
        (set `/Game/ThirdPerson/Blueprints/BP_ThirdPersonCharacter.ShotCount` 0.0 _char_ref)
        (`PrimitiveComponent.SetMaterial` (`self.playerLight`) 0 "/Game/StuffFromOGProject/SimonSaysPuzzle/simonSaysMaterials/Green_Mi.Green_Mi")
        (`GameplayStatics.PlaySoundAtLocation` "/Game/SoundEffects/gameStartSound.gameStartSound" (0.0 0.0 0.0) (struct) 1.0 1.0 0.0 null null null null)
        (`/Engine/EditorBlueprintResources/StandardMacros.IsValid` _returnvalue
          (:`Is Valid`
            (`self.DisableInput` _returnvalue)
            (`KismetSystemLibrary.Delay` 1.0)
            (`GameplayStatics.PlaySound2D` "/Game/MilitaryWeapSilver/Sound/GrenadeLauncher/Cues/GrenadeLauncher_Warning_Cue.GrenadeLauncher_Warning_Cue" 1.0 1.0 0.0 null null)
            (if (`self.IsflashbangEnabled`)
              (message `/Game/Widgets/Interface_Flashbang.Flashbang` (`self.Char Ref`))
              (`KismetSystemLibrary.Delay` 3.0)
              (bind _returnvalue_2 (`|SpawnActorFromClass` "/Game/ThirdPerson/Blueprints/BP_SingleTarget.BP_SingleTarget_C" (`KismetMathLibrary.Conv_VectorToTransform` (`KismetMathLibrary.RandomPointInBoundingBox` (`KismetMathLibrary.MakeVector` _returnvalue_x (+ _returnvalue_y 250.0) (+ _returnvalue_z 300.0)) (150.0 150.0 100.0))) "AdjustIfPossibleButAlwaysSpawn" "MultiplyWithRoot" null null))
              (`/Engine/EditorBlueprintResources/StandardMacros.IsValid` _returnvalue_2
                (:`Is Valid`
                  (`PrimitiveComponent.SetMaterial` (`self.playerLight`) 0 "/Game/StuffFromOGProject/SimonSaysPuzzle/simonSaysMaterials/Red_Mi.Red_Mi"))))))))))

(event `self.trigger.OnComponentBeginOverlap`
  (params (OverlappedComponent :type "PrimitiveComponent Object Reference") (OtherActor :type "Actor Object Reference") (OtherComp :type "PrimitiveComponent Object Reference") (OtherBodyIndex :type Integer) (bFromSweep :type Boolean) (SweepResult :type "HitResult Structure (by ref)"))
  (bind _asbp_third_person_character (cast `/Game/ThirdPerson/Blueprints/BP_ThirdPersonCharacter` OtherActor))
  (set `self.char Ref` _asbp_third_person_character)
  (`self.EnableInput` (`GameplayStatics.GetPlayerController` 0))
  (goto _label :!via `Open`))

(event `self.trigger.OnComponentEndOverlap`
  (params (OverlappedComponent :type "PrimitiveComponent Object Reference") (OtherActor :type "Actor Object Reference") (OtherComp :type "PrimitiveComponent Object Reference") (OtherBodyIndex :type Integer))
  (bind _asbp_third_person_character (cast `/Game/ThirdPerson/Blueprints/BP_ThirdPersonCharacter` OtherActor))
  (set `self.char Ref` _asbp_third_person_character)
  (`self.DisableInput` (`GameplayStatics.GetPlayerController` 0))
  (goto _label :!via `Close`))

(fn `UserConstructionScript`)