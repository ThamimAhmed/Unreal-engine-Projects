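; Hard-difficulty target spawner that starts a shooting round when the player presses Interact inside its trigger volume.
; Trigger overlaps store the character reference, toggle input and open or close a gate around the Interact event.
; Starting resets the character's score stats, shows the points widget, plays a sound, turns the light green and disables input.
; After a delay it spawns a random number of targets in an offset box, counting successful spawns and turning the light red.
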(event `EnhancedInput|/Game/ThirdPerson/Input/Actions/IA_Interact`
  (params (ActionValue :type Boolean) (ElapsedSeconds :type "Float (double-precision)") (TriggeredSeconds :type "Float (double-precision)") (InputAction :type "InputAction Object Reference" :default "/Game/ThirdPerson/Input/Actions/IA_Interact.IA_Interact"))
  (bind (_returnvalue_x _returnvalue_y _returnvalue_z) (`KismetMathLibrary.BreakVector` (`self.K2_GetActorLocation`)))
  (bind _returnvalue (`GameplayStatics.GetPlayerController` 0))
  (bind _maxtargetamount (`self.MaxTargetAmount`))
  (bind _char_ref (`self.char Ref`))
  (bind _mintargetamount (`self.MinTargetAmount`))
  (bind _returnvalue_2 (`KismetMathLibrary.RandomPointInBoundingBox` (`KismetMathLibrary.MakeVector` _returnvalue_x (+ _returnvalue_y 250.0) (+ _returnvalue_z 300.0)) (100.0 100.0 100.0)))
  ;[1 1 1] Trigger to spawn floating targets
  (:`Completed`
    (`/Engine/EditorBlueprintResources/StandardMacros.Gate` true :!label _label
      (:`Exit`
        (`UserWidget.AddToViewport` (`/Game/ThirdPerson/Blueprints/BP_ThirdPersonCharacter.PointsWidgetRef` (`self.Char Ref`)) 0)
        (set `/Game/ThirdPerson/Blueprints/BP_ThirdPersonCharacter.points` 0 _char_ref)
        (set `/Game/ThirdPerson/Blueprints/BP_ThirdPersonCharacter.Accuracy` 100.0 _char_ref)
        (set `/Game/ThirdPerson/Blueprints/BP_ThirdPersonCharacter.TotalShotsFired` 0.0 _char_ref)
        (set `/Game/ThirdPerson/Blueprints/BP_ThirdPersonCharacter.ShotsMissed` 0.0 _char_ref)
        (set `/Game/ThirdPerson/Blueprints/BP_ThirdPersonCharacter.ShotCount` 0.0 _char_ref)
        (`PrimitiveComponent.SetMaterial` (`self.playerLight`) 0 "/Game/StuffFromOGProject/SimonSaysPuzzle/simonSaysMaterials/Green_Mi.Green_Mi")
        (`GameplayStatics.PlaySoundAtLocation` "/Game/SoundEffects/gameStartSound.gameStartSound" (0.0 0.0 0.0) (struct) 1.0 1.0 0.0 null null null null)
        (`/Engine/EditorBlueprintResources/StandardMacros.IsValid` _returnvalue
          (:`Is Valid`
            (`self.DisableInput` _returnvalue)
            (`KismetSystemLibrary.Delay` 1.0)
            (bind _output_get (set `/Game/ThirdPerson/Blueprints/BP_ThirdPersonCharacter.TargetCount` 0 (`self.char Ref`)))
            ;[1 1 1] first index needs to be 1
            (for _index (range 1 (+ (`KismetMathLibrary.RandomIntegerInRange` _mintargetamount _maxtargetamount) 1))
              (`KismetSystemLibrary.PrintString` (`KismetStringLibrary.Conv_IntToString` _mintargetamount) false true (struct :`R` 1.0 :`G` 0.692669 :`A` 1.0) 2.0 "Min Target Amount")
              (`KismetSystemLibrary.PrintString` (`KismetStringLibrary.Conv_IntToString` _maxtargetamount) false true (struct :`G` 0.205502 :`B` 1.0 :`A` 1.0) 2.0 "max  target amount")
              (`KismetSystemLibrary.PrintString` (`KismetStringLibrary.Conv_IntToString` _index) false true (struct :`G` 1.0 :`B` 0.194544 :`A` 1.0) 2.0 "ActualAmount")
              (`KismetSystemLibrary.PrintString` (`KismetStringLibrary.Conv_VectorToString` _returnvalue_2) false true (struct :`R` 0.538562 :`B` 1.0 :`A` 1.0) 2.0 "point on bounding box")
              (bind _returnvalue_3 (`|SpawnActorFromClass` "/Game/ThirdPerson/Blueprints/BP_HardDifficultyTarget.BP_HardDifficultyTarget_C" (`KismetMathLibrary.Conv_VectorToTransform` _returnvalue_2) "AdjustIfPossibleButDontSpawnIfColliding" "MultiplyWithRoot" null null))
              (`/Engine/EditorBlueprintResources/StandardMacros.IsValid` _returnvalue_3
                (:`Is Valid`
                  (bind _result (`/Engine/EditorBlueprintResources/StandardMacros.IncrementInt` _output_get)
                    (:`  `
                      (bind _output_get_2 (set `/Game/ThirdPerson/Blueprints/BP_ThirdPersonCharacter.TargetCount` _result (`self.char Ref`)))
                      (`KismetSystemLibrary.PrintString` (`KismetStringLibrary.Conv_IntToString` _output_get_2) false true (struct :`R` 1.0 :`G` 0.935357 :`A` 1.0) 5.0)
                      (if (not (== _output_get_2 0))
                        (`PrimitiveComponent.SetMaterial` (`self.playerLight`) 0 "/Game/StuffFromOGProject/SimonSaysPuzzle/simonSaysMaterials/Red_Mi.Red_Mi")))))))))))))

(event `self.trigger.OnComponentBeginOverlap`
  (params (OverlappedComponent :type "PrimitiveComponent Object Reference") (OtherActor :type "Actor Object Reference") (OtherComp :type "PrimitiveComponent Object Reference") (OtherBodyIndex :type Integer) (bFromSweep :type Boolean) (SweepResult :type "HitResult Structure (by ref)"))
  ;[1 1 1] Trigger to spawn floating targets
  (bind _asbp_third_person_character (cast `/Game/ThirdPerson/Blueprints/BP_ThirdPersonCharacter` OtherActor))
  (set `self.char Ref` _asbp_third_person_character)
  (`self.EnableInput` (`GameplayStatics.GetPlayerController` 0))
  (goto _label :!via `Open`))

(event `self.trigger.OnComponentEndOverlap`
  (params (OverlappedComponent :type "PrimitiveComponent Object Reference") (OtherActor :type "Actor Object Reference") (OtherComp :type "PrimitiveComponent Object Reference") (OtherBodyIndex :type Integer))
  ;[1 1 1] Trigger to spawn floating targets
  (bind _asbp_third_person_character (cast `/Game/ThirdPerson/Blueprints/BP_ThirdPersonCharacter` OtherActor))
  (set `self.char Ref` _asbp_third_person_character)
  (`self.DisableInput` (`GameplayStatics.GetPlayerController` 0))
  (goto _label :!via `Close`))

(fn `UserConstructionScript`)