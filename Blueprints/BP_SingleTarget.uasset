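; Single shootable target that measures the player's reaction time from its spawn to the gun hit.
; BeginPlay stamps the start time in the third-person character's ReactionTimer after a zero-length delay.
; OnGunHit destroys the target, turns that timer into elapsed time and shows it on the reaction-time text actor.
; It also turns both scenario actors' player lights blue and enables input on the flashbang scenario, but calls the second EnableInput on itself.
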(event `self.ReceiveBeginPlay`
  (bind _asbp_third_person_character (cast `/Game/ThirdPerson/Blueprints/BP_ThirdPersonCharacter` (`GameplayStatics.GetPlayerCharacter` 0)))
  (bind _output_get (set `self.Char Ref` _asbp_third_person_character))
  (`KismetSystemLibrary.Delay` 0.0)
  (set `/Game/ThirdPerson/Blueprints/BP_ThirdPersonCharacter.ReactionTimer` (`GameplayStatics.GetUnpausedTimeSeconds`) _output_get))

(event `OnGunHit`
  (bind _returnvalue (`GameplayStatics.GetPlayerController` 0))
  (`self.K2_DestroyActor`)
  (bind _output_get (set `/Game/ThirdPerson/Blueprints/BP_ThirdPersonCharacter.ReactionTimer` (- (`GameplayStatics.GetUnpausedTimeSeconds`) (`/Game/ThirdPerson/Blueprints/BP_ThirdPersonCharacter.ReactionTimer` (`self.Char Ref`))) (`self.Char Ref`)))
  (bind _returnvalue_2 (`GameplayStatics.GetActorOfClass` "/Game/ThirdPerson/Blueprints/BP_ReactionTimeText.BP_ReactionTimeText_C"))
  (`TextRenderComponent.K2_SetText` (`/Game/ThirdPerson/Blueprints/BP_ReactionTimeText.ReactionTimeNo` _returnvalue_2) (`KismetTextLibrary.Conv_DoubleToText` _output_get "HalfToEven"))
  (`|ExecutionSequence`
    (:`then_0`
      (`KismetSystemLibrary.PrintString` (`KismetStringLibrary.Conv_DoubleToString` _output_get) false)
      (bind _returnvalue_3 (`GameplayStatics.GetActorOfClass` "/Game/ThirdPerson/Blueprints/BP_FlashbangScenario.BP_FlashbangScenario_C"))
      (`PrimitiveComponent.SetMaterial` (`/Game/ThirdPerson/Blueprints/BP_FlashbangScenario.playerLight` _returnvalue_3) 0 "/Game/StuffFromOGProject/SimonSaysPuzzle/simonSaysMaterials/Blue_Mi.Blue_Mi")
      (`/Engine/EditorBlueprintResources/StandardMacros.IsValid` _returnvalue
        (:`Is Valid`
          (`self.EnableInput` _returnvalue_3 _returnvalue))))
    (:`then_1`
      (bind _returnvalue_4 (`GameplayStatics.GetActorOfClass` "/Game/ThirdPerson/Blueprints/BP_ReactionTimeScenario.BP_ReactionTimeScenario_C"))
      (`PrimitiveComponent.SetMaterial` (`/Game/ThirdPerson/Blueprints/BP_ReactionTimeScenario.playerLight` _returnvalue_4) 0 "/Game/StuffFromOGProject/SimonSaysPuzzle/simonSaysMaterials/Blue_Mi.Blue_Mi")
      (`/Engine/EditorBlueprintResources/StandardMacros.IsValid` _returnvalue_4
        (:`Is Valid`
          (`self.EnableInput` (`GameplayStatics.GetPlayerController` 0)))))))

(fn `UserConstructionScript`)