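; Shooting-range target that slides side to side between its spawn point and a Y offset using two chained timelines, loading saved high scores on spawn.
; A delay started from the movement update destroys it after a timeout, resetting the player's points and target count.
; Gun hits add points and destroy it; the last one turns the BP_TargetSpawner light blue, re-enables its input and saves score and accuracy if both match or beat the records.
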(event `self.ReceiveBeginPlay`
  (bind (_returnvalue_x _returnvalue_y _returnvalue_z) (`KismetMathLibrary.BreakVector` (`self.K2_GetActorLocation`)))
  (bind _character_ref (`self.Character REF`))
  (bind _character_ref_2 (`self.Character REF`))
  (set `self.Start` (`KismetMathLibrary.MakeVector` _returnvalue_x _returnvalue_y _returnvalue_z))
  (set `self.End` (`KismetMathLibrary.MakeVector` _returnvalue_x (- _returnvalue_y 500.0) _returnvalue_z))
  (bind _asbp_third_person_character (cast `/Game/ThirdPerson/Blueprints/BP_ThirdPersonCharacter` (`GameplayStatics.GetPlayerCharacter` 0)))
  (set `self.Character REF` _asbp_third_person_character)
  ;[1 1 1] Loads Save Game to Set high score
  (bind _returnvalue (`GameplayStatics.DoesSaveGameExist` (`self.SlotName`)))
  (if _returnvalue
    (bind _returnvalue_2 (`GameplayStatics.LoadGameFromSlot` (`self.SlotName`)))
    (bind _output_get (set `self.SaverSubClass` _returnvalue_2))
    (bind _ashs (cast `/Game/ThirdPerson/Blueprints/HS` _output_get))
    (set `/Game/ThirdPerson/Blueprints/BP_ThirdPersonCharacter.Highscore` (`/Game/ThirdPerson/Blueprints/HS.Highscore` _ashs) _character_ref_2)
    (set `/Game/ThirdPerson/Blueprints/BP_ThirdPersonCharacter.AccuracyHighscore` (`/Game/ThirdPerson/Blueprints/HS.AccuracyHighscore` _ashs) _character_ref_2)
    ;[1 1 1] Timeline To move targets back and forth
    (bind (_direction _move) (`Timeline|Move` :!label _label)
      (:`Update`
        (`self.K2_SetActorRelativeLocation` (`KismetMathLibrary.VLerp` (`self.Start`) (`self.End`) _move))
        ;[1 1 1] After Some time, targets are destroyed
        (`KismetSystemLibrary.Delay` 15.0)
        (`self.K2_DestroyActor`)
        (set `/Game/ThirdPerson/Blueprints/BP_ThirdPersonCharacter.points` 0 _character_ref)
        (set `/Game/ThirdPerson/Blueprints/BP_ThirdPersonCharacter.TargetCount` 0 _character_ref)
        (bind _returnvalue_3 (`GameplayStatics.GetActorOfClass` "/Game/ThirdPerson/Blueprints/BP_TargetSpawner.BP_TargetSpawner_C"))
        (`PrimitiveComponent.SetMaterial` (`/Game/ThirdPerson/Blueprints/BP_TargetSpawner.playerLight` _returnvalue_3) 0 "/Game/StuffFromOGProject/SimonSaysPuzzle/simonSaysMaterials/Blue_Mi.Blue_Mi")
        (`GameplayStatics.PlaySoundAtLocation` "/Game/SoundEffects/gameStopSound.gameStopSound" (0.0 0.0 0.0) (struct) 1.0 1.0 0.0 null null null null))
      (:`Finished`
        (bind (_direction_2 _move_2) (`Timeline|Move_Back` :!via `ReverseFromEnd`)
          (:`Update`
            (`self.K2_SetActorRelativeLocation` (`KismetMathLibrary.VLerp` (`self.Start`) (`self.End`) _move_2)))
          (:`Finished`
            (goto _label :!via `PlayFromStart`)))))
    (else
      (goto _label))))

(event `OnGunHit`
  (bind _returnvalue (`GameplayStatics.GetPlayerController` 0))
  (bind _character_ref (`self.Character REF`))
  (bind _saversubclass (`self.SaverSubClass`))
  (bind _slotname (`self.SlotName`))
  (bind _character_ref_2 (`self.Character REF`))
  (bind _character_ref_3 (`self.Character REF`))
  (bind _accuracy (`/Game/ThirdPerson/Blueprints/BP_ThirdPersonCharacter.Accuracy` _character_ref_2))
  (bind _points (`/Game/ThirdPerson/Blueprints/BP_ThirdPersonCharacter.points` _character_ref_2))
  (set `self.IsHit` true)
  (set `/Game/ThirdPerson/Blueprints/BP_ThirdPersonCharacter.points` (+ (`/Game/ThirdPerson/Blueprints/BP_ThirdPersonCharacter.points` _character_ref_3) 10) _character_ref_3)
  (`self.K2_DestroyActor`)
  (set `/Game/ThirdPerson/Blueprints/BP_ThirdPersonCharacter.ShotCount` 0.0 (`self.Character REF`))
  (bind _output_get (set `/Game/ThirdPerson/Blueprints/BP_ThirdPersonCharacter.TargetCount` (- (`/Game/ThirdPerson/Blueprints/BP_ThirdPersonCharacter.TargetCount` _character_ref) 1) _character_ref))
  (`KismetSystemLibrary.PrintString` (`KismetStringLibrary.Conv_IntToString` _output_get) false)
  (if (== _output_get 0)
    (bind _returnvalue_2 (`GameplayStatics.GetActorOfClass` "/Game/ThirdPerson/Blueprints/BP_TargetSpawner.BP_TargetSpawner_C"))
    (`PrimitiveComponent.SetMaterial` (`/Game/ThirdPerson/Blueprints/BP_TargetSpawner.playerLight` _returnvalue_2) 0 "/Game/StuffFromOGProject/SimonSaysPuzzle/simonSaysMaterials/Blue_Mi.Blue_Mi")
    (`/Engine/EditorBlueprintResources/StandardMacros.IsValid` _returnvalue
      (:`Is Valid`
        (`self.EnableInput` _returnvalue_2 _returnvalue)
        ;[1 1 1] Saving
        (if (and (>= _points (`/Game/ThirdPerson/Blueprints/BP_ThirdPersonCharacter.Highscore` _character_ref_2)) (>= _accuracy (`/Game/ThirdPerson/Blueprints/BP_ThirdPersonCharacter.AccuracyHighscore` _character_ref_2)))
          (bind _output_get_2 (set `/Game/ThirdPerson/Blueprints/BP_ThirdPersonCharacter.Highscore` _points _character_ref_2))
          (bind _output_get_3 (set `/Game/ThirdPerson/Blueprints/BP_ThirdPersonCharacter.AccuracyHighscore` _accuracy _character_ref_2))
          (bind _returnvalue_3 (`GameplayStatics.DoesSaveGameExist` (`self.SlotName`)))
          (if _returnvalue_3
            (bind _returnvalue_4 (`GameplayStatics.LoadGameFromSlot` (`self.SlotName`)))
            (bind _output_get_4 (set `self.SaverSubClass` _returnvalue_4))
            (bind _ashs (cast `/Game/ThirdPerson/Blueprints/HS` _output_get_4))
            (set `/Game/ThirdPerson/Blueprints/HS.Highscore` _output_get_2 _ashs)
            (set `/Game/ThirdPerson/Blueprints/HS.AccuracyHighscore` _output_get_3 _ashs)
            (`GameplayStatics.SaveGameToSlot` _saversubclass _slotname)
            (else
              (bind _returnvalue_5 (`GameplayStatics.CreateSaveGameObject` "/Game/ThirdPerson/Blueprints/HS.HS_C"))
              (bind _output_get_5 (set `self.SaverSubClass` _returnvalue_5))
              (bind _ashs_2 (cast `/Game/ThirdPerson/Blueprints/HS` _output_get_5))
              (set `/Game/ThirdPerson/Blueprints/HS.Highscore` _output_get_2 _ashs_2)
              (set `/Game/ThirdPerson/Blueprints/HS.AccuracyHighscore` _output_get_3 _ashs_2)
              (`GameplayStatics.SaveGameToSlot` _saversubclass _slotname))))))
    (else
      (bind _returnvalue_6 (`GameplayStatics.GetActorOfClass` "/Game/ThirdPerson/Blueprints/BP_TargetSpawner.BP_TargetSpawner_C"))
      (`PrimitiveComponent.SetMaterial` (`/Game/ThirdPerson/Blueprints/BP_TargetSpawner.playerLight` _returnvalue_6) 0 "/Game/StuffFromOGProject/SimonSaysPuzzle/simonSaysMaterials/Red_Mi.Red_Mi")
      (`KismetSystemLibrary.PrintString` (`KismetStringLibrary.Conv_IntToString` (`/Game/ThirdPerson/Blueprints/BP_ThirdPersonCharacter.TargetCount` (`self.Character REF`))) false true (struct :`G` 0.66 :`B` 1.0 :`A` 1.0) 10.0))))

(fn `UserConstructionScript`)